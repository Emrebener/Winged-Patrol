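; BP_Menu is a world-space menu actor that hosts a menu widget and moves the player's view between linked menu actors.
; On BeginPlay it binds to the transition event of its Widget_MenuBase widget, which passes an index into the LinkedMenus array.
; A valid index disables this actor's collision, enables the target menu's collision and smoothly blends the player's view target to that menu.
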(event `self.ReceiveBeginPlay`
  (bind _aswidget_menu_base (cast `/Game/Blueprints/Menus/Widgets/Widget_MenuBase` (`WidgetComponent.GetUserWidgetObject` (`self.Widget`))))
  ;[1 1 1] binding an event for when this gets called
  (add `/Game/Blueprints/Menus/Widgets/Widget_MenuBase.TransitionToLinkedMenu` _aswidget_menu_base (delegate `OnTransitionBetweenMenus`)))

(event `OnTransitionBetweenMenus`
  (params (MenuIndex :type Integer))
  (if (`KismetArrayLibrary.Array_IsValidIndex` (`self.LinkedMenus`) MenuIndex)
    (`self.transitionTo` (`|GetArrayItem` (`self.LinkedMenus`) MenuIndex))))

(event `transitionTo`
  (params (NewMenu :type "/Blueprints/Menus/BP_Menu Object Reference"))
  (`self.SetActorEnableCollision` false)
  (`self.SetActorEnableCollision` NewMenu true)
  (`PlayerController.SetViewTargetWithBlend` (`GameplayStatics.GetPlayerController` 0) NewMenu 2.0 "VTBlend_EaseInOut" 2.0 false))

(fn `UserConstructionScript`)