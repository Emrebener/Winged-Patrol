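; Tree actor for a wildfire game that gets a random cedar mesh and can burn, spread fire or be extinguished.
; After a startup delay it caches neighboring trees overlapping its propagation sphere.
; While burning, a looping timer ignites one random neighbor that is neither burning nor previously extinguished.
; It updates fire counts in BP_MyGameMode, triggering a loss when too many trees burn and a win when none remain alight.
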(event `self.ReceiveBeginPlay`
  (bind _asbp_my_game_mode (cast `/Game/Blueprints/BP_MyGameMode` (`GameplayStatics.GetGameMode`)))
  (set `self.RefToGameMode` _asbp_my_game_mode)
  ;[0.5842 0.4927 1 1 24] when the game starts, find the neighboring trees for each tree and store it in an array
  (`KismetSystemLibrary.Delay` 2.0)
  (for _array_element (`PrimitiveComponent.GetOverlappingActors` (`self.FirePropogationSphere`) "BP_MyNewTree_C")
    (bind _asbp_my_new_tree (cast `/Blueprints/MyTree/MyTrees/BP_MyNewTree` _array_element))
    (`KismetArrayLibrary.Array_Add` (`self.NeighborTrees`) _asbp_my_new_tree)))

(fn `canBeSetOnFire`
  (params (`Input Tree` :type "/Blueprints/MyTree/MyTrees/BP_MyNewTree Object Reference"))
  (returns (ReturnValue :type Boolean))
  (return (`KismetMathLibrary.BooleanNOR` (`/Blueprints/MyTree/MyTrees/BP_MyNewTree.IsOnFire` `Input Tree`) (`/Blueprints/MyTree/MyTrees/BP_MyNewTree.BeenExtinguished` `Input Tree`))))

(fn `extinguish`
  ;[0.3478 1 0.7112 1 24] extinguish
  (set `self.IsOnFire` false)
  (set `self.BeenExtinguished` true)
  (`ActorComponent.Deactivate` (`self.FireParticleSystem`))
  (`KismetSystemLibrary.K2_ClearTimer` null "spreadFire")
  (`/Engine/EditorBlueprintResources/StandardMacros.IncrementInt` (`/Game/Blueprints/BP_MyGameMode.TreesExtinguished` (`self.RefToGameMode`))
    (:`  `
      (bind _result (`/Engine/EditorBlueprintResources/StandardMacros.DecrementInt` (`/Game/Blueprints/BP_MyGameMode.TreesOnFire` (`self.RefToGameMode`)))
        (:`  `
          (if (== _result 0)
            (`/Game/Blueprints/BP_MyGameMode.WinGame` (`self.RefToGameMode`))))))))

(fn `setOnFire`
  ;[1 0.4279 0.528 1 24] set on fire
  (set `self.IsOnFire` true)
  (`ActorComponent.Activate` (`self.FireParticleSystem`) false)
  (`/Engine/EditorBlueprintResources/StandardMacros.IncrementInt` (`/Game/Blueprints/BP_MyGameMode.TreesOnFire` (`self.RefToGameMode`))
    (:`  `
      (`KismetSystemLibrary.K2_SetTimer` null "spreadFire" (`self.FirePropogationSpeed`) true)
      (if (> (`/Game/Blueprints/BP_MyGameMode.TreesOnFire` (`self.RefToGameMode`)) 60)
        (set `/Game/Blueprints/BP_MyGameMode.LosingReason` "wildfire spreaded too much!" (`self.RefToGameMode`))
        (`/Game/Blueprints/BP_MyGameMode.LoseGame` (`self.RefToGameMode`))))))

(fn `spreadFire`
  (`KismetSystemLibrary.PrintString` (`KismetStringLibrary.Concat_StrStr` (`KismetSystemLibrary.GetDisplayName` self) " is attempting to spread fire...") true true (struct :`R` 1.0 :`G` 0.132347 :`B` 0.202059 :`A` 1.0) 4.0)
  (for _array_element (`self.NeighborTrees`)
    ;[0.9879 1 0.4779] process each neighbor tree to check which ones can be set on fire
    (if (`self.canBeSetOnFire` _array_element)
      (`KismetArrayLibrary.Array_Add` (`self.AvailableNeighborTrees`) _array_element)))
  ;[1 0.4317 0.3719 1 24] if there are any available neighbor tree to be set on fire, set a random one of them on fire
  (if (not (`self.isArrayEmpty` (`self.AvailableNeighborTrees`)))
    (`self.setOnFire` (`KismetArrayLibrary.Array_Random` (`self.AvailableNeighborTrees`)))
    (`KismetArrayLibrary.Array_Clear` (`self.AvailableNeighborTrees`))
    (`KismetSystemLibrary.PrintString` (`KismetStringLibrary.Concat_StrStr` (`KismetSystemLibrary.GetDisplayName` self) " spreaded it's fire!") true true (struct :`G` 1.0 :`B` 0.14985 :`A` 1.0) 4.0)))

(fn `UserConstructionScript`
  ;[0.6244 1 0.7891 1 24] assign a random mesh to the tree
  (switch `int` (`KismetMathLibrary.RandomIntegerInRange` 0 2)
    (:`0`
      ;;[0.6004 0.5714 1 1 24] cedar large
      (`StaticMeshComponent.SetStaticMesh` (`self.TreeMesh`) "/Game/Brushify/Meshes/Foliage/Trees/Cedar/S_Cedar_Large.S_Cedar_Large"))
    (:`1`
      ;;[0.6004 0.5714 1 1 24] cedar medium
      (`StaticMeshComponent.SetStaticMesh` (`self.TreeMesh`) "/Game/Brushify/Meshes/Foliage/Trees/Cedar/S_Cedar_Medium.S_Cedar_Medium"))
    (:`2`
      ;;[0.6004 0.5714 1 1 24] cedar small
      (`StaticMeshComponent.SetStaticMesh` (`self.TreeMesh`) "/Game/Brushify/Meshes/Foliage/Trees/Cedar/S_Cedar_Small.S_Cedar_Small"))))