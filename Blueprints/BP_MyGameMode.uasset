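; Game mode Blueprint that handles the end of a match with win and lose outcomes.
; WinGame and LoseGame each pause the game, switch the first player controller to Game and UI input, and show the mouse cursor.
; Each then creates its own result widget, the winning or losing screen, and adds it to the viewport.
; Nothing in this graph triggers either function, as BeginPlay and Tick are empty.
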(fn `LoseGame`
  (`GameplayStatics.SetGamePaused` true)
  (`WidgetBlueprintLibrary.SetInputMode_GameAndUIEx` (`GameplayStatics.GetPlayerController` 0) null)
  (set `PlayerController.bShowMouseCursor` true (`GameplayStatics.GetPlayerController` 0))
  (bind _returnvalue (`|CreateWidget` "/Game/Blueprints/Menus/Widgets/Widget_LoseScreen.Widget_LoseScreen_C"))
  (`UserWidget.AddToViewport` _returnvalue 0))

(fn `UserConstructionScript`)

(fn `WinGame`
  (`GameplayStatics.SetGamePaused` true)
  (`WidgetBlueprintLibrary.SetInputMode_GameAndUIEx` (`GameplayStatics.GetPlayerController` 0) null)
  (set `PlayerController.bShowMouseCursor` true (`GameplayStatics.GetPlayerController` 0))
  (bind _returnvalue (`|CreateWidget` "/Game/Blueprints/Menus/Widgets/Widget_WinningScreen.Widget_WinningScreen_C"))
  (`UserWidget.AddToViewport` _returnvalue 0))